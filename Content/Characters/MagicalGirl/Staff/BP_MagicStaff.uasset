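; BP_MagicStaff is a magic staff pickup with an animated orb and two rings.
; Tick and SequencerTick share the same rotation logic, so it also animates under Sequencer, spinning the orb on yaw and the rings in opposite directions.
; The rotation steps are fixed per frame, not scaled by delta time.
; When the player character overlaps the capsule, it calls AddSpecialMessage on that character and destroys itself.
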(event OnComponentBeginOverlap(Capsule)
  (params (OverlappedComponent :type Primitive%20Component%20Object%20Reference) (OtherActor :type Actor%20Object%20Reference) (OtherComp :type Primitive%20Component%20Object%20Reference) (OtherBodyIndex :type Integer) (bFromSweep :type Boolean) (SweepResult :type Hit%20Result%20Structure%20%28by%20ref%29))
  (bind _returnvalue (Game|GetPlayerCharacter 0))
  (if (== OtherActor _returnvalue)
    (Class|IFPickup|AddSpecial(Message) _returnvalue)
    (Actor|DestroyActor)))

(event Custom|SequencerTick
  (Transformation|AddLocalRotation (Variables|Default|GetOrb) (Math|Rotator|MakeRotator 0.0 0.0 0.5) false true)
  (Transformation|AddLocalRotation (Variables|Default|GetOrb_ring) (Math|Rotator|MakeRotator -0.5 0.5 0.0) false true)
  (Transformation|AddLocalRotation (Variables|Default|GetOrb_ring_2) (Math|Rotator|MakeRotator 0.5 -0.5 0.0) false true))

(event EventTick
  (params (DeltaSeconds :type Float%20%28single-precision%29))
  (Transformation|AddLocalRotation (Variables|Default|GetOrb) (Math|Rotator|MakeRotator 0.0 0.0 0.5) false true)
  (Transformation|AddLocalRotation (Variables|Default|GetOrb_ring) (Math|Rotator|MakeRotator -0.5 0.5 0.0) false true)
  (Transformation|AddLocalRotation (Variables|Default|GetOrb_ring_2) (Math|Rotator|MakeRotator 0.5 -0.5 0.0) false true))

(fn ConstructionScript)