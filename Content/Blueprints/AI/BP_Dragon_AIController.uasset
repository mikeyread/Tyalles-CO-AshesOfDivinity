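; AI controller for the dragon that runs Dragon_BT and switches it into hunting when it perceives the player.
; BeginPlay and Possess start the tree; a target perception update for BP_PlayerPawn sets blackboard Enemy and Should hunt, gated by a flag that is never re-armed here.
; A custom event clears Should hunt.
; Tick prints that value for debugging, and the general perception-update loop is empty.
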(event OnTargetPerceptionUpdated(AIPerception)
  (params (Actor :type Actor%20Object%20Reference) (Stimulus :type AI%20Stimulus%20Structure))
  (bind _asbp_player_pawn (Utilities|Casting|CastToBP_PlayerPawn Actor))
  (if (Variables|Default|GetNewVar)
    (Variables|Default|SetNewVar false)
    (AI|Components|Blackboard|SetValueasObject (AI|GetBlackboard 0) (Utilities|Name|MakeLiteralName "Enemy") _asbp_player_pawn)
    (AI|Components|Blackboard|SetValueasBool (AI|GetBlackboard 0) (Utilities|Name|MakeLiteralName "Should hunt") true)))

(event OnPerceptionUpdated(AIPerception)
  (params (UpdatedActors :type Array%20of%20Actor%20Object%20References))
  (Utilities|FlowControl|Sequence
    (:then_0
      (for _array_element UpdatedActors
        _))))

(event Custom|CustomEvent
  (AI|Components|Blackboard|SetValueasBool (AI|GetBlackboard 0) (Utilities|Name|MakeLiteralName "Should hunt") false))

(event EventTick
  (params (DeltaSeconds :type Float%20%28single-precision%29))
  (Development|PrintString (Utilities|String|ToString(Boolean) (ScalableFloat|GetValueasBool (AI|GetBlackboard 0) (Utilities|Name|MakeLiteralName "Should hunt")))))

(event EventPossess
  (params (PossessedPawn :type Pawn%20Object%20Reference))
  (AI|RunBehaviorTree "/Game/Blueprints/AI/Dragon_BT.Dragon_BT"))

(event EventBeginPlay
  (AI|RunBehaviorTree "/Game/Blueprints/AI/Dragon_BT.Dragon_BT"))

(fn ConstructionScript)